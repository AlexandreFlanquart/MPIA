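; BP_House is a static mesh actor that switches color between red and blue whenever another actor begins overlapping it.
; The construction script creates a dynamic material instance on the mesh and sets its P_Color parameter to red.
; Each overlap prints a debug message, flips IsBlue and plays one of two color timelines, BlueToRed or RedToBlue, which drive P_Color on the mesh's materials.
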(event EventBeginPlay)

(event Collision|EventActorBeginOverlap
  (params (OtherActor :type Actor%20Object%20Reference))
  ;[1 1 1] Switch color
  (Development|PrintString "Collide")
  (bind _output_get (Variables|Default|SetisBlue (not (Variables|Default|GetisBlue))))
  (if _output_get
    (bind _bluetored (Timeline|Timeline PlayFromStart)
      (:Update
        (Rendering|Material|SetVectorParameterValueonMaterials (Variables|Default|GetStaticMesh) "P_Color" (Math|Conversions|ToVector(LinearColor) _bluetored))))
    (else
      (bind _redtoblue (Timeline|Timeline_0 PlayFromStart)
        (:Update
          (Rendering|Material|SetVectorParameterValueonMaterials (Variables|Default|GetStaticMesh) "P_Color" (Math|Conversions|ToVector(LinearColor) _redtoblue)))))))

(event EventTick
  (params (DeltaSeconds :type Float%20%28single-precision%29)))

(fn ConstructionScript
  (bind _returnvalue (Rendering|Material|CreateDynamicMaterialInstance (Variables|Default|GetStaticMesh) 0 0 "None" :!class /Script/Engine.PrimitiveComponent))
  (Rendering|Material|SetVectorParameterValue _returnvalue "P_Color" (Variables|Default|GetredColor) :!class /Script/Engine.MaterialInstanceDynamic)
  (Variables|Default|SetcurrentColor (Variables|Default|GetredColor)))